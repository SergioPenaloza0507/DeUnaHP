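; FallingCharacter is a character steered by bursts from a physics thruster while the Fire input is held.
; On press, it deprojects the mouse position, flattens it to the actor's height, sets the thruster's relative rotation facing away from that point, then activates it.
; Releasing Fire or a touch deactivates the thruster.
; A touch-based version of the aiming logic is left unconnected, so touch cannot start thrust.
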(event EventBeginPlay)

(event Collision|EventActorBeginOverlap
  (params (OtherActor :type Actor%20Object%20Reference)))

(event EventTick
  (params (DeltaSeconds :type Float%20%28single-precision%29)))

(event Input|ActionEvents|InputActionFire
  (params (Key :type Key%20Structure))
  (bind _returnvalue (Game|GetPlayerController 0))
  (bind _returnvalue_2 (Transformation|GetActorLocation))
  (bind _physicsthruster (Variables|Default|GetPhysicsThruster))
  (bind (_locationx _locationy) (Game|Player|GetMousePosition _returnvalue))
  (bind _returnvalue_3 (Math|Vector2D|MakeVector2D _locationx _locationy))
  (bind _worldposition (Class|GameplayStatics|DeprojectScreentoWorld _returnvalue _returnvalue_3))
  (bind (_x _y) (Math|Vector|BreakVector _worldposition))
  (:Pressed
    (Transformation|SetRelativeRotation _physicsthruster (Math|Rotator|FindLookatRotation _returnvalue_2 (+ _returnvalue_2 (Math|Vector|Normalize (- _returnvalue_2 (Math|Vector|MakeVector _x _y (.Z (Math|Vector|BreakVector _returnvalue_2))))))) false false)
    (Components|Activation|Activate _physicsthruster false))
  (:Released
    (Components|Activation|Deactivate _physicsthruster)))

(event Input|TouchEvents|InputTouch
  (params (Location :type Vector) (FingerIndex :type ETouchIndex%20Enum))
  (:Released
    (Components|Activation|Deactivate (Variables|Default|GetPhysicsThruster))))

(fn ConstructionScript)